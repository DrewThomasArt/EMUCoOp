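; Function library for touch-driven character rotation in HeroSelectPro, with helpers that track touches on BPI_Rotate widgets and rotate meshes.
; Press picks the last-listed widget under the touch, testing only horizontal bounds, and records it by finger index in a touch-info array.
; Press, move and release update that array and message all canvas children with DPI-scaled positions.
; Separate helpers add inverted, scaled yaw to a mesh or set its relative rotation.
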(fn `AddWidgetArray`
  (params (CanvasPanel :type "PanelWidget Object Reference") (TargetArray :type "Array of Widget Object Reference (by ref)"))
  ;[0 0 0] Add all childrens of main panel to WidgetAry
  (for _index (range (`PanelWidget.GetChildrenCount` CanvasPanel))
    (bind _returnvalue (`PanelWidget.GetChildAt` CanvasPanel _index))
    (if (`KismetSystemLibrary.DoesImplementInterface` _returnvalue "/Game/HeroSelectPro/Blueprints/BPI_Rotate.BPI_Rotate_C")
      (`KismetArrayLibrary.Array_Add` TargetArray _returnvalue))))

(fn `ConverToWidgetLoc`
  (params (Location :type "Vector Structure"))
  (returns (WidgetLoc2D :type "Vector2D Structure"))
  (return (`KismetMathLibrary.MakeVector2D` (.x (/ Location (`WidgetLayoutLibrary.GetViewportScale` null))) (.y (/ Location (`WidgetLayoutLibrary.GetViewportScale` null))))))

(fn `FindTouchInfo_ButtonRef`
  (params (WidgetRef :type "Widget Object Reference") (TouchInfoAry :type "Array of /Game/HeroSelectPro/Blueprints/ST_WidgetRotateInfo Structure"))
  (returns (IsFind :type Boolean) (Result :type "/Game/HeroSelectPro/Blueprints/ST_WidgetRotateInfo Structure"))
  (for _array_element TouchInfoAry
    (if (== (`.WidgetRef_2_4C5D87CE4BD74295D5FBC7A9EBC88EE0` (break `/Game/HeroSelectPro/Blueprints/ST_WidgetRotateInfo` _array_element)) WidgetRef)
      (return true _array_element)))
  (return false))

(fn `FindTouchInfoArray`
  (params (FingerIndex :type Byte) (TouchInfoArray :type "Array of /Game/HeroSelectPro/Blueprints/ST_WidgetRotateInfo Structure"))
  (returns (Result :type "Array of Integer"))
  (locals (LocalTouchInfoAry :type "Array of  Structure") (LocalIndexAry :type "Array of Integer"))
  (for (_array_element _array_index) TouchInfoArray
    (if (== (`.FingerIndex_7_2A28C38A465EE70CB7C0D894A0699489` (break `/Game/HeroSelectPro/Blueprints/ST_WidgetRotateInfo` _array_element)) FingerIndex)
      (`KismetArrayLibrary.Array_Add` (`local.LocalIndexAry`) _array_index)))
  (return (`local.LocalIndexAry`)))

(fn `GetScreenSize`
  (returns (ReturnValue :type "Vector2D Structure"))
  (bind _returnvalue (`WidgetLayoutLibrary.GetViewportScale` null))
  (bind (_x _y) (`KismetMathLibrary.BreakVector2D` (`WidgetLayoutLibrary.GetViewportSize` null)))
  (return (`KismetMathLibrary.MakeVector2D` (/ _x _returnvalue) (/ _y _returnvalue))))

(fn `IsPointInButton`
  (params (IpPoint :type "Vector Structure") (IpButtonRef :type "Widget Object Reference"))
  (returns (Result :type Boolean))
  (locals (LocalPoint :type "Vector Structure") (LocalScreenSize :type "Vector2D Structure") (LocalAnchorMinPoint :type "Vector2D Structure") (LocalPosition :type "Vector2D Structure") (LocalSize :type "Vector2D Structure") (IpButtonRef_L :type "Widget Object Reference"))
  (bind _x (.x IpPoint))
  (bind _returnvalue (* (`WidgetLayoutLibrary.GetViewportScale` null) (`KismetMathLibrary.BreakVector2D` (`local.LocalPosition`))))
  (set `local.IpButtonRef_L` IpButtonRef)
  (`|ExecutionSequence`
    (:`then_0`
      ;[0 0 0] Calculate Button location
      (bind _returnvalue_2 (`self.GetScreenSize` null))
      (bind _output_get (set `local.LocalScreenSize` _returnvalue_2))
      (set `local.LocalAnchorMinPoint` (* _output_get (`.Minimum` (break `Anchors` (`CanvasPanelSlot.GetAnchors` (`WidgetLayoutLibrary.SlotAsCanvasSlot` (`local.IpButtonRef_L`)))))))
      (set `local.LocalPosition` (+ (`CanvasPanelSlot.GetPosition` (`WidgetLayoutLibrary.SlotAsCanvasSlot` (`local.IpButtonRef_L`))) (`local.LocalAnchorMinPoint`)))
      (set `local.LocalSize` (`CanvasPanelSlot.GetSize` (`WidgetLayoutLibrary.SlotAsCanvasSlot` (`local.IpButtonRef_L`)))))
    (:`then_1`
      (return (and (>= _x _returnvalue) (<= _x (+ _returnvalue (* (`WidgetLayoutLibrary.GetViewportScale` null) (`KismetMathLibrary.BreakVector2D` (`local.LocalSize`))))))))))

(fn `MeshRotation`
  (params (Mesh :type "SceneComponent Object Reference") (Axis :type "Float (double-precision)") (valueRotation :type "Float (double-precision)"))
  (bind (_returnvalue_roll _returnvalue_pitch _returnvalue_yaw) (`KismetMathLibrary.BreakRotator` (`KismetMathLibrary.MakeRotator` 0.0 0.0 Axis)))
  (`SceneComponent.K2_AddRelativeRotation` Mesh (`KismetMathLibrary.MakeRotator` 0.0 0.0 (* (* _returnvalue_yaw valueRotation) -1.0)) false false))

(fn `OnMovedTouch`
  (params (Location :type "Vector Structure") (FingerIndex :type Byte) (TouchInfoArrayT :type "Array of /Game/HeroSelectPro/Blueprints/ST_WidgetRotateInfo Structure") (CanvasPanel :type "CanvasPanel Object Reference"))
  (locals (MoveTouchPrev :type "Vector Structure") (MovedPointTouch :type "Vector Structure"))
  (bind _movedpointtouch (`local.MovedPointTouch`))
  (set `local.MoveTouchPrev` (`local.MovedPointTouch`))
  (set `local.MovedPointTouch` Location)
  (for _array_element (`self.FindTouchInfoArray` FingerIndex TouchInfoArrayT)
    (bind _structout (setmembers `/Game/HeroSelectPro/Blueprints/ST_WidgetRotateInfo` :`StructRef` (`|GetArrayItem` TouchInfoArrayT _array_element) :`Location` _movedpointtouch :`Loc2D_WidgetSpace` (`self.ConverToWidgetLoc` _movedpointtouch)))
    (for _index (range (`PanelWidget.GetChildrenCount` CanvasPanel))
      (bind ((`WidgetRef_2_4C5D87CE4BD74295D5FBC7A9EBC88EE0` _widgetref) (`Loc2D_WidgetSpace_17_B4B5B96C431A8F68ACD2DCBE3D484B2D` _loc2d_widgetspace)) (break `/Game/HeroSelectPro/Blueprints/ST_WidgetRotateInfo` _structout))
      (message `/Game/HeroSelectPro/Blueprints/BPI_Rotate.OnWidgetMoved_Touch` (`PanelWidget.GetChildAt` CanvasPanel _index) _widgetref _loc2d_widgetspace))))

(fn `OnPressedTouch`
  (params (PressedTouchPoint :type "Vector Structure") (FingerIndex :type Byte) (WidgetArray :type "Array of Widget Object Reference") (`TouchInfoArray ` :type "Array of /Game/HeroSelectPro/Blueprints/ST_WidgetRotateInfo Structure") (`CanvasPanel_Main ` :type "CanvasPanel Object Reference"))
  (bind _widgetloc2d (`self.ConverToWidgetLoc` PressedTouchPoint))
  ;[0 0 0] Get and Set Rotate Widget
  (bind (_ispick _resultwidgetary) (`self.PickWidget` PressedTouchPoint WidgetArray))
  (if _ispick
    (for _array_element _resultwidgetary
      ;[0 0 0] Check if PickWidetRef dose not contain in TouchInfoAry
      (if (not (`self.FindTouchInfo_ButtonRef` _array_element `TouchInfoArray `))
        (bind _st_widgetrotateinfo (make `/Game/HeroSelectPro/Blueprints/ST_WidgetRotateInfo` _array_element FingerIndex PressedTouchPoint PressedTouchPoint _widgetloc2d _widgetloc2d))
        ;[0 0 0] Add TouchInfo to TouchInfoAry
        (`KismetArrayLibrary.Array_Add` `TouchInfoArray ` _st_widgetrotateinfo)
        (for _index (range (`PanelWidget.GetChildrenCount` `CanvasPanel_Main `))
          (bind ((`WidgetRef_2_4C5D87CE4BD74295D5FBC7A9EBC88EE0` _widgetref) (`PressedLoc2D_WidgetSpace_15_C7E2D42C447FBBC5961609A5705F9D6F` _pressedloc2d_widgetspace)) (break `/Game/HeroSelectPro/Blueprints/ST_WidgetRotateInfo` _st_widgetrotateinfo))
          (message `/Game/HeroSelectPro/Blueprints/BPI_Rotate.OnWidgetPressed_Touch` (`PanelWidget.GetChildAt` `CanvasPanel_Main ` _index) _widgetref _pressedloc2d_widgetspace))))))

(fn `OnReleasedTouch`
  (params (InputPin :type Byte) (TouchInfoArray :type "Array of /Game/HeroSelectPro/Blueprints/ST_WidgetRotateInfo Structure") (CanvasPanel :type "PanelWidget Object Reference"))
  (bind _removetouchinfoary (`self.RemoveTouchInfo_FingerIndex` InputPin TouchInfoArray))
  (for _array_element _removetouchinfoary
    (for _index (range (`PanelWidget.GetChildrenCount` CanvasPanel))
      (bind ((`WidgetRef_2_4C5D87CE4BD74295D5FBC7A9EBC88EE0` _widgetref) (`Loc2D_WidgetSpace_17_B4B5B96C431A8F68ACD2DCBE3D484B2D` _loc2d_widgetspace)) (break `/Game/HeroSelectPro/Blueprints/ST_WidgetRotateInfo` _array_element))
      (message `/Game/HeroSelectPro/Blueprints/BPI_Rotate.OnWidgetReleased_Touch` (`PanelWidget.GetChildAt` CanvasPanel _index) _widgetref _loc2d_widgetspace))))

(fn `PickWidget`
  (params (PickLoc :type "Vector Structure") (WidgetAry :type "Array of Widget Object Reference"))
  (returns (IsPick :type Boolean) (ResultWidgetAry :type "Array of Widget Object Reference"))
  (locals (LocalWidget :type "Widget Object Reference") (LocalWidgetAry :type "Array of Widget Object Reference"))
  (bind (_arrayindex _arrayelement) (`/Engine/EditorBlueprintResources/StandardMacros.ReverseForEachLoop` WidgetAry)
    (:`LoopBody`
      (set `local.LocalWidget` _arrayelement)
      (if (`self.IsPointInButton` PickLoc (`local.LocalWidget`))
        (`KismetArrayLibrary.Array_Add` (`local.LocalWidgetAry`) (`local.LocalWidget`))
        (return true (`local.LocalWidgetAry`))))
    (:`Completed`
      (return false (`local.LocalWidgetAry`)))))

(fn `RemoveTouchInfo`
  (params (IpWidget :type "Widget Object Reference") (FingerIndex :type Byte) (TouchInfoAry :type "Array of /Game/HeroSelectPro/Blueprints/ST_WidgetRotateInfo Structure"))
  (for (_array_element _array_index) TouchInfoAry
    (bind ((`WidgetRef_2_4C5D87CE4BD74295D5FBC7A9EBC88EE0` _widgetref) (`FingerIndex_7_2A28C38A465EE70CB7C0D894A0699489` _fingerindex)) (break `/Game/HeroSelectPro/Blueprints/ST_WidgetRotateInfo` _array_element))
    (if (and (== _widgetref IpWidget) (== _fingerindex FingerIndex))
      (`KismetArrayLibrary.Array_Remove` TouchInfoAry _array_index)
      (break))))

(fn `RemoveTouchInfo_FingerIndex`
  (params (FingerIndex :type Byte) (TouchInfoAry :type "Array of /Game/HeroSelectPro/Blueprints/ST_WidgetRotateInfo Structure"))
  (returns (RemoveTouchInfoAry :type "Array of /Game/HeroSelectPro/Blueprints/ST_WidgetRotateInfo Structure"))
  (locals (LocalArrayIndexAry :type "Array of Integer") (LocalTouchInfo :type "/Game/HeroSelectPro/Blueprints/ST_WidgetRotateInfo Structure") (LocalTouchInfoArray :type "Array of /Game/HeroSelectPro/Blueprints/ST_WidgetRotateInfo Structure"))
  (for (_array_element _array_index) TouchInfoAry
    (set `local.LocalTouchInfo` _array_element)
    (if (== (`.FingerIndex_7_2A28C38A465EE70CB7C0D894A0699489` (break `/Game/HeroSelectPro/Blueprints/ST_WidgetRotateInfo` _array_element)) FingerIndex)
      (`KismetArrayLibrary.Array_Add` (`local.LocalArrayIndexAry`) _array_index)
      (`KismetArrayLibrary.Array_Add` (`local.LocalTouchInfoArray`) (`local.LocalTouchInfo`))))
  (for _array_element_2 (`local.LocalTouchInfoArray`)
    (bind ((`WidgetRef_2_4C5D87CE4BD74295D5FBC7A9EBC88EE0` _widgetref) (`FingerIndex_7_2A28C38A465EE70CB7C0D894A0699489` _fingerindex)) (break `/Game/HeroSelectPro/Blueprints/ST_WidgetRotateInfo` _array_element_2))
    (`self.RemoveTouchInfo` _widgetref _fingerindex TouchInfoAry))
  (return (`local.LocalTouchInfoArray`)))

(fn `Setting Rotation`
  (params (`Update?` :type Boolean) (Mesh :type "SceneComponent Object Reference") (NewRotation :type "Rotator Structure"))
  (returns (`Rotación relativa` :type "Rotator Structure"))
  (if `Update?`
    (`SceneComponent.K2_SetRelativeRotation` Mesh NewRotation false false)
    (else
      (return (`SceneComponent.RelativeRotation` Mesh)))))