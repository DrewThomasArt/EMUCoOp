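; Function library for a hero selection system, shared by the selection screen and gameplay.
; Reads character rows through DT_System and persists the chosen character and lock state in SG_SelectCharacter slots, defaulting to the configured starting character.
; Applies each row's mesh, select or gameplay animation class, and optional material with a timed color effect.
; Also creates and toggles voice and particle components, and switches camera view targets.
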(fn `ActiveSound_System`
  (params (`Active?` :type Boolean) (ComponentsVoice :type "AudioComponent Object Reference") (StartTime :type "Float (double-precision)"))
  (if `Active?`
    (`/Engine/EditorBlueprintResources/StandardMacros.IsValid` ComponentsVoice
      (:`Is Valid`
        (`AudioComponent.Play` ComponentsVoice StartTime)))
    (else
      (`/Engine/EditorBlueprintResources/StandardMacros.IsValid` ComponentsVoice
        (:`Is Valid`
          (`AudioComponent.Stop` ComponentsVoice))))))

(fn `ActiveVFX_System`
  (params (`Active?` :type Boolean) (FVX :type "ActorComponent Object Reference"))
  (`/Engine/EditorBlueprintResources/StandardMacros.IsValid` FVX
    (:`Is Valid`
      (if `Active?`
        (`ActorComponent.Activate` FVX true)
        (else
          (`ActorComponent.Deactivate` FVX))))))

(fn `Buttons To Array `
  (params (`BTN RZW` :type "/Game/HeroSelectPro/Widgets/WBP_BaseBTNCharacter Object Reference (by ref)") (TargetArray :type "Array of /Game/HeroSelectPro/Widgets/WBP_BaseBTNCharacter Object Reference (by ref)"))
  (`KismetArrayLibrary.Array_Insert` TargetArray `BTN RZW` (`/Game/HeroSelectPro/Widgets/WBP_BaseBTNCharacter.NroBTN` `BTN RZW`)))

(fn `ChangeCameraControl`
  (params (CameraComp :type "ActorComponent Object Reference"))
  ;[0 0 0] change camera control
  (`PlayerController.SetViewTargetWithBlend` (`GameplayStatics.GetPlayerController` null) (`ActorComponent.GetOwner` CameraComp) 0.5 "VTBlend_Linear" 0.0 true)
  (`Controller.SetControlRotation` (`GameplayStatics.GetPlayerController` null) (`Actor.K2_GetActorRotation` (`ActorComponent.GetOwner` CameraComp)))
  (`WidgetBlueprintLibrary.SetInputMode_GameOnly` (`GameplayStatics.GetPlayerController` null)))

(fn `CreateComponentsFVX`
  (params (DataCharacter :type "/Game/HeroSelectPro/Blueprints/ST_ListCharacters Structure") (AttachToComponent :type "SceneComponent Object Reference"))
  (returns (Output_Comp_FVX_StarT :type "ParticleSystemComponent Object Reference") (Output_Comp_FVX_SelectT :type "ParticleSystemComponent Object Reference"))
  (locals (Data_T :type "/Game/HeroSelectPro/Blueprints/ST_ListCharacters Structure") (Comp_FVX_StarT :type "ParticleSystemComponent Object Reference") (Comp_FVX_SelectT :type "ParticleSystemComponent Object Reference"))
  (bind ((`nameBone_FvxSelect_162_47C6092E4C9B2392DE2AB99ED30F0DEF` _namebone_fvxselect) (`FVX_Select_163_8548AAC043513D5FBCC1ED9C80708341` _fvx_select) (`FVX_Select_Location_178_9045133E4D1C047D318DB99D741BE64D` _fvx_select_location) (`FVX_Select_Rotation_180_E6E391AF41E96D15A1463281663088AA` _fvx_select_rotation) (`FVX_Select_Scale_170_D2E982634151AF1F6989BC9945520D25` _fvx_select_scale)) (break `/Game/HeroSelectPro/Blueprints/ST_ListCharacters` (`local.Data_T`)))
  (bind ((`nameBone_FvxStar_160_3FC33E5C4E2D58FEB2B35CAF84981405` _namebone_fvxstar) (`Fvx_Star_51_826B7D124FB171587304EC995DB4FA5E` _fvx_star) (`FVX_Star_Location_177_5C4E6D4B417AD1ACFAFF4B8F20929B13` _fvx_star_location) (`FVX_Star_Rotation_179_7C88637B499A129E9C104DBEDB3C1FA0` _fvx_star_rotation) (`FVX_Star_Scale_168_4E9D3C484C6EE8444543CCAA5368CED1` _fvx_star_scale)) (break `/Game/HeroSelectPro/Blueprints/ST_ListCharacters` (`local.Data_T`)))
  (set `local.Data_T` DataCharacter)
  (`/Engine/EditorBlueprintResources/StandardMacros.IsValid` _fvx_star
    (:`Is Valid`
      ;[0 0 0] Setup Sparks Left Foot
      (bind _returnvalue (`GameplayStatics.SpawnEmitterAttached` _fvx_star AttachToComponent _namebone_fvxstar _fvx_star_location _fvx_star_rotation _fvx_star_scale "KeepRelativeOffset" false "None" false))
      (bind _output_get (set `local.Comp_FVX_StarT` _returnvalue))
      (`ActorComponent.Deactivate` _output_get))
    (:`Is Not Valid`
      (set `local.Comp_FVX_StarT` null)))
  ;[0 0 0] Setup Sparks Right Foot
  (`/Engine/EditorBlueprintResources/StandardMacros.IsValid` _fvx_select
    (:`Is Valid`
      (bind _returnvalue_2 (`GameplayStatics.SpawnEmitterAttached` _fvx_select AttachToComponent _namebone_fvxselect _fvx_select_location _fvx_select_rotation _fvx_select_scale "KeepRelativeOffset" false "None" false))
      (bind _output_get_2 (set `local.Comp_FVX_SelectT` _returnvalue_2))
      (`ActorComponent.Deactivate` _output_get_2))
    (:`Is Not Valid`
      (set `local.Comp_FVX_SelectT` null)))
  (return (`local.Comp_FVX_StarT`) (`local.Comp_FVX_SelectT`)))

(fn `CreateComponentsSVX`
  (params (DataCharacter :type "/Game/HeroSelectPro/Blueprints/ST_ListCharacters Structure"))
  (returns (Output_ComponentVoiceStar :type "AudioComponent Object Reference") (Output_ComponentsVoiceSelect :type "AudioComponent Object Reference"))
  (locals (Data_T :type "/Game/HeroSelectPro/Blueprints/ST_ListCharacters Structure") (ComponentVoiceStarT :type "AudioComponent Object Reference") (ComponentVoiceSelectT :type "AudioComponent Object Reference"))
  (bind ((`icon_Character404x602_190_49B3469E4E0C1016B35A898B8F3A8BC4` _icon_character404x602) (`Svx_StarTime_VoiceStar_186_4BC41A3A40183B8988E4A2AB391E1695` _svx_startime_voicestar) (`Svx_CharacterVoiceSelect_157_085FDA68444EEE1071CA9A93735606A0` _svx_charactervoiceselect)) (break `/Game/HeroSelectPro/Blueprints/ST_ListCharacters` (`local.Data_T`)))
  (bind ((`icon_Character404x602_190_49B3469E4E0C1016B35A898B8F3A8BC4` _icon_character404x602_2) (`Svx_CharacterVoiceStar_156_6F2B96234706F19AB5718DABAB9BE608` _svx_charactervoicestar)) (break `/Game/HeroSelectPro/Blueprints/ST_ListCharacters` (`local.Data_T`)))
  (set `local.Data_T` DataCharacter)
  (`/Engine/EditorBlueprintResources/StandardMacros.IsValid` _svx_charactervoicestar
    (:`Is Valid`
      (bind _returnvalue (`GameplayStatics.CreateSound2D` null _svx_charactervoicestar 1.0 1.0 0.0 null false false))
      (set `local.ComponentVoiceStarT` _returnvalue))
    (:`Is Not Valid`
      (set `local.ComponentVoiceStarT` null)))
  (`/Engine/EditorBlueprintResources/StandardMacros.IsValid` _svx_charactervoiceselect
    (:`Is Valid`
      (bind _returnvalue_2 (`GameplayStatics.CreateSound2D` null _svx_charactervoiceselect 1.0 1.0 0.0 null false false))
      (set `local.ComponentVoiceSelectT` _returnvalue_2))
    (:`Is Not Valid`
      (set `local.ComponentVoiceSelectT` null)))
  (return (`local.ComponentVoiceStarT`) (`local.ComponentVoiceSelectT`)))

(fn `Get Data Character`
  (params (nroPersonaje :type Integer))
  (returns (SelectCharacter :type "/Game/HeroSelectPro/Blueprints/ST_ListCharacters Structure"))
  ;[0 0 0] Load the information from the data table
  (bind _returnvalue (`|GetDataTableRow` "/Game/HeroSelectPro/DataTable/DT_System.DT_System" "1")
    (:`then`
      (bind _returnvalue_2 (`|GetDataTableRow` (`.DataCharacters_2_C6068A5F4B81F88B991FD09F30F9B10F` (break `/Game/HeroSelectPro/Blueprints/ST_DataSystem` _returnvalue)) (`KismetStringLibrary.Conv_StringToName` (`KismetStringLibrary.Conv_IntToString` nroPersonaje)))
        (:`then`
          (return _returnvalue_2))))))

(fn `Load Current Character`
  (returns (CodCurrentCharacter_S :type Integer) (`IsBlocked?_S` :type Boolean))
  (bind _slotname (`self.nameSlotSave` "NewEnumerator1"))
  (bind _returnvalue (`GameplayStatics.DoesSaveGameExist` _slotname))
  (if _returnvalue
    (bind _returnvalue_2 (`GameplayStatics.LoadGameFromSlot` _slotname))
    (bind _assg_select_character (cast `/Game/HeroSelectPro/Blueprints/SG_SelectCharacter` _returnvalue_2))
    (return (`/Game/HeroSelectPro/Blueprints/SG_SelectCharacter.CodCurrentCharacter_S` _assg_select_character) (`/Game/HeroSelectPro/Blueprints/SG_SelectCharacter.IsBlocked?_S` _assg_select_character))
    (else
      (bind _returnvalue_3 (`|GetDataTableRow` "/Game/HeroSelectPro/DataTable/DT_System.DT_System" "1")
        (:`then`
          (bind ((`StartingCharacterNumber_6_2B4AD2B5466D72661DDCDBA67F2AF2B8` _startingcharacternumber)) (break `/Game/HeroSelectPro/Blueprints/ST_DataSystem` _returnvalue_3))
          (`self.Save Current Character` _startingcharacternumber)
          (return _startingcharacternumber false))))))

(fn `Load3DCharacter`
  (returns (Character3DMesh :type "/Game/HeroSelectPro/Blueprints/BP_HeroSelect Object Reference") (CameraMainMenu :type "CameraActor Object Reference"))
  (bind _slotname (`self.nameSlotSave` "NewEnumerator0"))
  (bind _returnvalue (`GameplayStatics.DoesSaveGameExist` _slotname))
  (if _returnvalue
    (bind _returnvalue_2 (`GameplayStatics.LoadGameFromSlot` _slotname))
    (bind _assg_select_character (cast `/Game/HeroSelectPro/Blueprints/SG_SelectCharacter` _returnvalue_2))
    (return (`/Game/HeroSelectPro/Blueprints/SG_SelectCharacter.Character3DMesh` _assg_select_character) (`/Game/HeroSelectPro/Blueprints/SG_SelectCharacter.CameraMainMenu` _assg_select_character))))

(fn `LoadDataCharacter`
  (params (ST_ListCharacters :type "/Game/HeroSelectPro/Blueprints/ST_ListCharacters Structure (by ref)") (Mesh :type "SkeletalMeshComponent Object Reference") (`isPlayGame?` :type Boolean))
  (locals (MeshT :type "SkeletalMeshComponent Object Reference") (DataCharacterT :type "/Game/HeroSelectPro/Blueprints/ST_ListCharacters Structure"))
  (set `local.DataCharacterT` ST_ListCharacters)
  (set `local.MeshT` Mesh)
  (`SkinnedMeshComponent.SetSkinnedAssetAndUpdate` (`local.MeshT`) (`.3D_Mesh_58_AB47C7214A9785B84F580B8D664F76FC` (break `/Game/HeroSelectPro/Blueprints/ST_ListCharacters` (`local.DataCharacterT`))) true)
  (if `isPlayGame?`
    (`SkeletalMeshComponent.SetAnimInstanceClass` (`local.MeshT`) (`.BP_AnimationPlayGame_145_4706C3F94212165A1F508F9391CEB2F6` (break `/Game/HeroSelectPro/Blueprints/ST_ListCharacters` (`local.DataCharacterT`))))
    (else
      (`SkeletalMeshComponent.SetAnimInstanceClass` (`local.MeshT`) (`.BP_AnimationSelect_56_B33E2ED84874110AB4419D94953C0A8D` (break `/Game/HeroSelectPro/Blueprints/ST_ListCharacters` (`local.DataCharacterT`))))))
  (if (`.MaterialBasedChange?_73_1DC9D84248A406494972B8A4DE217B70` (break `/Game/HeroSelectPro/Blueprints/ST_ListCharacters` (`local.DataCharacterT`)))
    (`PrimitiveComponent.SetMaterial` (`local.MeshT`) 0 (`.Material_76_1F67A5F245C310519E1FFD832CF2C577` (break `/Game/HeroSelectPro/Blueprints/ST_ListCharacters` (`local.DataCharacterT`))))
    (`self.PlayMaterialEffects` (struct :`R` 1.0 :`G` 0.928537 :`B` 0.358333 :`A` 1.0) (`local.MeshT`))))

(fn `nameSlotSave`
  (params (Selection :type "/Game/HeroSelectPro/Blueprints/BP_E_TypeSaveData Enum" :default "NewEnumerator0"))
  (returns (slotName :type String))
  (switch `/Game/HeroSelectPro/Blueprints/BP_E_TypeSaveData` Selection
    (:`NewEnumerator0`
      (return "Save3DCharacter"))
    (:`NewEnumerator1`
      (return "DataSelectCharacter"))))

(fn `PlayMaterialEffects`
  (params (ColorLineal :type "LinearColor Structure") (Mesh :type "SkeletalMeshComponent Object Reference"))
  (`MeshComponent.SetVectorParameterValueOnMaterials` Mesh "EffectColor" (`KismetMathLibrary.Conv_LinearColorToVector` ColorLineal))
  (`MeshComponent.SetScalarParameterValueOnMaterials` Mesh "StartTime" (`GameplayStatics.GetTimeSeconds` null)))

(fn `Save Current Character`
  (params (`Cod Current Character` :type Integer) (PurchaseStatus :type Boolean))
  (locals (CodCurrent_S :type Integer) (PurchaseStatusS :type Boolean))
  (set `local.CodCurrent_S` `Cod Current Character`)
  (set `local.PurchaseStatusS` PurchaseStatus)
  (bind _returnvalue (`GameplayStatics.CreateSaveGameObject` "/Game/HeroSelectPro/Blueprints/SG_SelectCharacter.SG_SelectCharacter_C"))
  (set `/Game/HeroSelectPro/Blueprints/SG_SelectCharacter.CodCurrentCharacter_S` (`local.CodCurrent_S`) _returnvalue)
  (set `/Game/HeroSelectPro/Blueprints/SG_SelectCharacter.IsBlocked?_S` (`local.PurchaseStatusS`) _returnvalue)
  (`GameplayStatics.SaveGameToSlot` _returnvalue (`self.nameSlotSave` "NewEnumerator1")))

(fn `Save3DCharacter`
  (params (Character3DMesh :type "/Game/HeroSelectPro/Blueprints/BP_HeroSelect Object Reference") (CameraMainMenuRef :type "CameraActor Object Reference"))
  (locals (BPCharacter3DMeshT :type "/Game/HeroSelectPro/Blueprints/BP_HeroSelect Object Reference") (CameraMainMenuT :type "CameraActor Object Reference"))
  (set `local.BPCharacter3DMeshT` Character3DMesh)
  (set `local.CameraMainMenuT` CameraMainMenuRef)
  (`CameraComponent.SetConstraintAspectRatio` (`CameraActor.CameraComponent` CameraMainMenuRef) false)
  (`PlayerController.SetViewTargetWithBlend` (`GameplayStatics.GetPlayerController` null) (`local.CameraMainMenuT`) 0.0 "VTBlend_Linear" 0.0 false)
  (`PlayerController.SetVirtualJoystickVisibility` (`GameplayStatics.GetPlayerController` null) false)
  (bind _returnvalue (`GameplayStatics.DoesSaveGameExist` (`self.nameSlotSave` "NewEnumerator0")))
  (if (not _returnvalue)
    (bind _returnvalue_2 (`GameplayStatics.CreateSaveGameObject` "/Game/HeroSelectPro/Blueprints/SG_SelectCharacter.SG_SelectCharacter_C"))
    (set `/Game/HeroSelectPro/Blueprints/SG_SelectCharacter.Character3DMesh` (`local.BPCharacter3DMeshT`) _returnvalue_2)
    (set `/Game/HeroSelectPro/Blueprints/SG_SelectCharacter.CameraMainMenu` (`local.CameraMainMenuT`) _returnvalue_2)
    (`GameplayStatics.SaveGameToSlot` _returnvalue_2 (`self.nameSlotSave` "NewEnumerator0"))))

(fn `SelectCharacterPlayGame`
  (params (Mesh :type "SkeletalMeshComponent Object Reference"))
  (`WidgetBlueprintLibrary.SetInputMode_GameOnly` (`GameplayStatics.GetPlayerController` null))
  (bind _codcurrentcharacter_s (`self.Load Current Character` null))
  (bind _selectcharacter (`self.Get Data Character` _codcurrentcharacter_s))
  (`self.LoadDataCharacter` _selectcharacter Mesh true))