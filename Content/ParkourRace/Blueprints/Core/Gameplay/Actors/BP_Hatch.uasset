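; BP_Hatch is a parkour hatch platform that swings open, then rotates back up after a random delay.
; With ReactToPlayerCollision set, a box overlap gives a coin-flip chance to drop it immediately; otherwise it cycles from BeginPlay with random pauses.
; Timelines drive the mesh's roll down and up, while ReadyForUse blocks retriggering until the reset finishes.
; Drop, reset and random logic run only on the server through authority checks.
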(event `self.ReceiveBeginPlay`
  (`/Engine/EditorBlueprintResources/ActorMacros.Switch Has Authority`
    (:`Authority`
      (if (not (`self.ReactToPlayerCollision?`))
        (`self.Hatch_Down`)))))

(event `self.Box.OnComponentBeginOverlap`
  (params (OverlappedComponent :type "PrimitiveComponent Object Reference") (OtherActor :type "Actor Object Reference") (OtherComp :type "PrimitiveComponent Object Reference") (OtherBodyIndex :type Integer) (bFromSweep :type Boolean) (SweepResult :type "HitResult Structure (by ref)"))
  ;[0.05098 0.05098 0.05098] Randomly Drop Hatch when the player jumps on the platform. (If 'ReactToPlayerCollision' = true )
  (`self.Randomly_DropHatch`))

(event `Hatch_Down`
  ;[0.05098 0.05098 0.05098] Random hatch behaviour
  (`/Engine/EditorBlueprintResources/ActorMacros.Switch Has Authority`
    (:`Authority`
      ;;[0.05098 0.05098 0.05098] Check if it's ready to drop the hatch again
      (if (`self.ReadyForUse?`)
        (set `self.ReadyForUse?` false)
        (if (`self.ReactToPlayerCollision?`)
          (bind (_direction _rotation) (`Timeline|Hatch_Rotate_Down` :!via `PlayFromStart` :!label _label)
            (:`Update`
              (`SceneComponent.K2_SetRelativeRotation` (`self.SM_Hatch`) (`KismetMathLibrary.MakeRotator` _rotation) false false))
            (:`Finished`
              (`self.Reset_Hatch`)))
          (else
            ;;[0.05098 0.05098 0.05098 1 16] Randomly rotate the hatch down
            (`KismetSystemLibrary.Delay` (`KismetMathLibrary.RandomFloatInRange` 1.0 3.0))
            (goto _label :!via `PlayFromStart`)))))))

(event `Reset_Hatch`
  ;[0.05098 0.05098 0.05098] Random hatch behaviour
  (`/Engine/EditorBlueprintResources/ActorMacros.Switch Has Authority`
    (:`Authority`
      ;;[0.05098 0.05098 0.05098 1 16] Randomly reset pillar
      (`KismetSystemLibrary.Delay` (`KismetMathLibrary.RandomFloatInRange` 1.0 3.0))
      ;;[0.05098 0.05098 0.05098] Resets the Hatch to upwards position
      (bind (_direction _rotation) (`Timeline|Hatch_Rotate_Up` :!via `PlayFromStart`)
        (:`Update`
          (`SceneComponent.K2_SetRelativeRotation` (`self.SM_Hatch`) (`KismetMathLibrary.MakeRotator` _rotation) false false))
        (:`Finished`
          (set `self.ReadyForUse?` true)
          (if (not (`self.ReactToPlayerCollision?`))
            (`self.Hatch_Down`)))))))

(fn `Randomly_DropHatch`
  (`/Engine/EditorBlueprintResources/ActorMacros.Switch Has Authority`
    (:`Authority`
      ;[0.05098 0.05098 0.05098] 50% chance the Hatch get's dropped
      (switch `int` (`KismetMathLibrary.RandomIntegerInRange` 0 1)
        (:`0`
          (`self.Hatch_Down`))))))

(fn `UserConstructionScript`)